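; Auto-turret cannon that turns toward and fires at NetCharacter actors inside its detection sphere.
; Sphere overlaps maintain the IncomingEnemies list, skipping the cannon's owner.
; Looping timers replace Tick, refreshing a raised muzzle location, calling CannonFireBullet per valid enemy, and yawing toward each in turn, leaving it facing the last.
; CannonAckEnemies is an unscheduled debug targeting variant, and the DebugArray timer event is empty.
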(event `Debug Array`
  ;[1 1 1] Debug
)

(event `self.ReceiveBeginPlay`
  (`KismetSystemLibrary.K2_SetTimerDelegate` (delegate `Get Muzzle Location`) 0.02 true)
  (`KismetSystemLibrary.K2_SetTimerDelegate` (delegate `Debug Array`) 0.2 true)
  (`KismetSystemLibrary.K2_SetTimerDelegate` (delegate `CannonFire`) 0.5 true)
  (`KismetSystemLibrary.K2_SetTimerDelegate` (delegate `CannonAttackEnemies`) 1.0 true))

(event `Get Muzzle Location`
  ;[1 1 1] 刷新炮口Location
  (`self.MuzzleLoc` (+ (`SceneComponent.K2_GetComponentLocation` (`self.Muzzle`)) (0.0 0.0 70.0))))

(event `CannonFire`
  ;[1 1 1] Fire Bullet
  (for _array_element (`self.IncomingEnemies`)
    (if (`KismetSystemLibrary.IsValid` _array_element)
      (`self.CannonFireBullet`))))

(event `CannonAttackEnemies`
  ;[1 1 1] Cannon Ack Enemies
  (for _array_element (`self.IncomingEnemies`)
    (if (`KismetSystemLibrary.IsValid` _array_element)
      (bind (_returnvalue_roll _returnvalue_pitch _returnvalue_yaw) (`KismetMathLibrary.BreakRotator` (`KismetMathLibrary.FindLookAtRotation` (`self.K2_GetActorLocation`) (`self.K2_GetActorLocation` _array_element))))
      (`self.K2_SetActorRotation` (`KismetMathLibrary.MakeRotator` 0.0 0.0 _returnvalue_yaw)))))

(event `self.Sphere.OnComponentBeginOverlap`
  (params (OverlappedComponent :type "PrimitiveComponent Object Reference") (OtherActor :type "Actor Object Reference") (OtherComp :type "PrimitiveComponent Object Reference") (OtherBodyIndex :type Integer) (bFromSweep :type Boolean) (SweepResult :type "HitResult Structure (by ref)"))
  ;[1 1 1] Overlap
  (if (not (== (`self.GetOwner`) OtherActor))
    (bind _asnet_character (cast `NetCharacter` OtherActor))
    (`KismetArrayLibrary.Array_Add` (`self.IncomingEnemies`) _asnet_character)))

(event `CannonAckEnemies`
  (bind _arrayhub (`self.ArrayHub`))
  ;[1 1 1] Debug Cannon
  (for (_array_element _array_index) (`self.IncomingEnemies`)
    (bind _output_get (set `self.ArrayHub` (+ _array_index _arrayhub)))
    (`KismetArrayLibrary.Array_Add` (`self.AttackTarget`) _array_element))
  (`KismetSystemLibrary.PrintString` (`KismetStringLibrary.Conv_IntToString` _arrayhub) true true (struct :`R` 1.0 :`B` 0.172555 :`A` 1.0) 0.2)
  (if (!= _output_get 0)
    (for _array_element_2 (`self.AttackTarget`)
      (bind (_returnvalue_roll _returnvalue_pitch _returnvalue_yaw) (`KismetMathLibrary.BreakRotator` (`KismetMathLibrary.FindLookAtRotation` (`self.K2_GetActorLocation`) (`self.K2_GetActorLocation` _array_element_2))))
      (`self.K2_SetActorRotation` (`KismetMathLibrary.MakeRotator` 0.0 0.0 _returnvalue_yaw))
      (set `self.ArrayHub` 0))))

(event `self.Sphere.OnComponentEndOverlap`
  (params (OverlappedComponent :type "PrimitiveComponent Object Reference") (OtherActor :type "Actor Object Reference") (OtherComp :type "PrimitiveComponent Object Reference") (OtherBodyIndex :type Integer))
  ;[1 1 1] Overlap
  (if (not (== (`self.GetOwner`) OtherActor))
    (bind _asnet_character (cast `NetCharacter` OtherActor))
    (`KismetArrayLibrary.Array_RemoveItem` (`self.IncomingEnemies`) _asnet_character)))

(fn `UserConstructionScript`)